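; BP_sleep is a trigger actor that sets the player controller's view target to the player character when that character enters its Box.
; BeginPlay caches the player as a HorrorEngineCharacter, and the Box overlap compares against that reference before calling SetViewTargetWithBlend.
; A Camera reference and an offset actor-location calculation sit unused in the graph, so no sleep behavior is implemented here.
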(event `self.ReceiveBeginPlay`
  (bind _ashorror_engine_character (cast `/Game/HorrorEngine/Blueprints/Core/HorrorEngineCharacter` (`GameplayStatics.GetPlayerCharacter` 0)))
  (set `self.Player` _ashorror_engine_character))

(event `self.Box.OnComponentBeginOverlap`
  (params (OverlappedComponent :type "PrimitiveComponent Object Reference") (OtherActor :type "Actor Object Reference") (OtherComp :type "PrimitiveComponent Object Reference") (OtherBodyIndex :type Integer) (bFromSweep :type Boolean) (SweepResult :type "HitResult Structure (by ref)"))
  (bind _player (`self.Player`))
  (if (== _player OtherActor)
    (`PlayerController.SetViewTargetWithBlend` (`GameplayStatics.GetPlayerController` 0) _player 0.0 "VTBlend_Linear" 0.0 false)))

(fn `UserConstructionScript`)