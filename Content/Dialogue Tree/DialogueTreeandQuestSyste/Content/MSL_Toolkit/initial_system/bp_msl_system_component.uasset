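; Player controller component that bootstraps the MSL toolkit on BeginPlay, intended to give each client its own copy of the system.
; It spawns localization and settings actors, then the dialogue control actor with dialogue, map and quest viewport widgets, and finally the savegame actor.
; Dialogue initializes before savegame so saved state loads afterward, existence checks avoid duplicates, and a loaded flag is set at the end.
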(event `self.ReceiveBeginPlay`
  ;[1 1 1] This component should spawn all important actors with game start,
  ; should be added to player controller only.
  ; beginplay is here.
  (`self.init_system`) ; this is only client sided call,\nbecause each client should have its own copy of system.
)

(event `init_system`
  ;[1 1 1] This component should spawn all important actors with game start,
  ; should be added to player controller only.
  ; beginplay is here.
  (`|ExecutionSequence`
    (:`then_0`
      (`self.init_spawn`))))

(fn `init_dlg`
  (locals (local_transform :type "Transform Structure"))
  ;[1 1 1] Init all dlg widgets and necessary actors.
  (`|ExecutionSequence`
    (:`then_0`
      (bind _outactors (`GameplayStatics.GetAllActorsOfClass` "/Game/DLG_Tree/dlg_system/blueprints/base/bp_dlg_control.bp_dlg_control_C"))
      (if (not (`KismetArrayLibrary.Array_IsValidIndex` _outactors))
        (bind _returnvalue (`|SpawnActorFromClass` "/Game/DLG_Tree/dlg_system/blueprints/base/bp_dlg_control.bp_dlg_control_C" (`local.local_transform`) "AlwaysSpawn" "OverrideRootScale" null null))
        (set `self.dlg_controls` _returnvalue)))
    (:`then_1`
      (`/Engine/EditorBlueprintResources/StandardMacros.IsValid` (`self.w_dlg_layout`)
        (:`Is Not Valid`
          (bind _returnvalue_2 (`|CreateWidget` "/Game/DLG_Tree/dlg_system/widgets/base/w_01_dlg_2d_layout.w_01_dlg_2d_layout_C"))
          (set `self.w_dlg_layout` _returnvalue_2)
          (`/Game/DLG_Tree/dlg_system/widgets/base/w_01_dlg_2d_layout.init_widget` (`self.w_dlg_layout`))
          (`UserWidget.AddToViewport` (`self.w_dlg_layout`) 0))))
    (:`then_2`
      (`/Engine/EditorBlueprintResources/StandardMacros.IsValid` (`self.w_map_layout`)
        (:`Is Not Valid`
          (bind _returnvalue_3 (`|CreateWidget` "/Game/DLG_Tree/dmap_system/widgets/w_01_map_layout.w_01_map_layout_C"))
          (set `self.w_map_layout` _returnvalue_3)
          (`/Game/DLG_Tree/dmap_system/widgets/w_01_map_layout.init_widget` (`self.w_map_layout`))
          (`UserWidget.AddToViewport` (`self.w_map_layout`) 0))))
    (:`then_3`
      (`/Engine/EditorBlueprintResources/StandardMacros.IsValid` (`self.w_quest_layout`)
        (:`Is Not Valid`
          (bind _returnvalue_4 (`|CreateWidget` "/Game/DLG_Tree/dqst_system/widgets/base/w_01_quest_layout.w_01_quest_layout_C"))
          (set `self.w_quest_layout` _returnvalue_4)
          (`/Game/DLG_Tree/dqst_system/widgets/base/w_01_quest_layout.init_widget` (`self.w_quest_layout`))
          (`UserWidget.AddToViewport` (`self.w_quest_layout`) 0))))))

(fn `init_spawn`
  (locals (local_transform :type "Transform Structure"))
  ;[1 1 1] This actor should init system and load all actors.
  (`|ExecutionSequence`
    (:`then_0`
      (`|ExecutionSequence`
        (:`then_0`
          (bind _outactors (`GameplayStatics.GetAllActorsOfClass` "/Game/MSL_Toolkit/localization_system/blueprints/bp_msl_localization_actor.bp_msl_localization_actor_C"))
          (if (not (`KismetArrayLibrary.Array_IsValidIndex` _outactors))
            (bind _returnvalue (`|SpawnActorFromClass` "/Game/MSL_Toolkit/localization_system/blueprints/bp_msl_localization_actor.bp_msl_localization_actor_C" (`local.local_transform`) "AlwaysSpawn" "OverrideRootScale" null null))
            (set `self.localization_actor` _returnvalue)))
        (:`then_1`
          (bind _outactors_2 (`GameplayStatics.GetAllActorsOfClass` "/Game/MSL_Toolkit/settings_system/blueprints/bp_msl_settings_actor.bp_msl_settings_actor_C"))
          (if (not (`KismetArrayLibrary.Array_IsValidIndex` _outactors_2))
            (bind _returnvalue_2 (`|SpawnActorFromClass` "/Game/MSL_Toolkit/settings_system/blueprints/bp_msl_settings_actor.bp_msl_settings_actor_C" (`local.local_transform`) "AlwaysSpawn" "OverrideRootScale" null null))
            (set `self.settings_actor` _returnvalue_2)))
        (:`then_2`
          (`self.init_dlg`) ; init dialogue widgets and etc before savegame,\nso the system will load them after the dialogue init.
        )
        (:`then_3`
          (bind _outactors_3 (`GameplayStatics.GetAllActorsOfClass` "/Game/MSL_Toolkit/savegame_system/blueprints/bp_msl_savegame_actor.bp_msl_savegame_actor_C"))
          (if (not (`KismetArrayLibrary.Array_IsValidIndex` _outactors_3))
            (bind _returnvalue_3 (`|SpawnActorFromClass` "/Game/MSL_Toolkit/savegame_system/blueprints/bp_msl_savegame_actor.bp_msl_savegame_actor_C" (`local.local_transform`) "AlwaysSpawn" "OverrideRootScale" null null))
            (set `self.savegame_actor` _returnvalue_3)))))
    (:`then_1`
      (set `self.is_system_loaded` true) ; after all necessary actors are spawned,\nand all objects is loaded from save file and etc,\nwe should mark the system as loaded.
    )))