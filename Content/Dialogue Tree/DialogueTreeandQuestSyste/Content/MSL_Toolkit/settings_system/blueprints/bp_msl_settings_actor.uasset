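; Settings actor for the MSL Toolkit that manages rebindable PC and gamepad input with localized key names and platform icons.
; On BeginPlay it builds axis and action bindings from DataTables, preferring the save file unless the binding count differs.
; Rebinding clears conflicts within the same category.
; ApplyInput rewrites engine InputSettings mappings at runtime by name or category, optionally resetting defaults or saving to settings and SaveGame.
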(event `self.ReceiveBeginPlay`
  ;[1 1 1] Init event,
  ; load the needed functions and apply settings.
  (`self.init_settings`))

(event `init_settings`
  ;[1 1 1] Init event,
  ; load the needed functions and apply settings.
  (`|ExecutionSequence`
    (:`then_0`
      (`self.create_keys_data`) ; first we create necessary keys data,\nwhich is needed for inputs/rebinds and etc.
      (`self.load_input` false) ; should load defaults to add categories and \nremove save file, if it's length is not equal to default.
    )
    (:`then_1`
      (`|ExecutionSequence`
        (:`then_0`
          (bind (_input_list _input_data) (`self.load_input` (`self.debug_apply_defaults`)))
          (set `self.input_list` _input_list)
          (set `self.input_data` _input_data))
        (:`then_1`
          (if (`self.apply_on_boot`)
            (`self.apply_input` "None" "None" true false true) ; Also apply input data of all categories,\nso it will directly get populated to project settings,\nand will work in game.
          ))))))

(fn `apply_input`
  (params (input_name :type Name) (input_category :type Name) (all_categories :type Boolean) (reset_defaults :type Boolean) (save_inputs :type Boolean))
  (locals (local_input_id :type Name) (local_input_index :type Integer) (local_positive_keys :type "Array of InputChord Structure") (local_negative_keys :type "Array of InputChord Structure") (local_action_keys :type "Array of InputChord Structure") (local_invalid_keys :type "Array of Key Structure") (local_input_list :type "Array of Name") (local_default_data :type "Array of /Game/MSL_Toolkit/settings_system/structs/s_input_data Structure"))
  (bind _local_input_index (`local.local_input_index`))
  (bind (_positive_keys _negative_keys _action_keys) (break `/Game/MSL_Toolkit/settings_system/structs/s_input_data` (`|GetArrayItem` (`self.input_data`) (`local.local_input_index`))))
  ;[1 1 1] this function does apply all the key inputs at runtime, so the changes are instantanously goes to gameplay,
  ; this does have features like to apply specific category of inputs or all categories, also reset the default input settings,
  ; and save the current input settings to file.
  (if (!= input_name "None")
    (set `local.local_input_list` (`|MakeArray` input_name))
    (else
      (bind _input_list (`self.get_inputs_by_category` input_category all_categories))
      (set `local.local_input_list` _input_list)))
  ;[1 1 1] if input is going to reset, load the defaults value data, and hold it as local array.
  (if (`local.reset_defaults`)
    (bind (_input_list_2 _input_data) (`self.load_input` true))
    (set `local.local_default_data` _input_data))
  ;[1 1 1] loop for all input filtered by categories, and check if they are valid to process.
  (for _array_element (`local.local_input_list`)
    (bind _output_get (set `local.local_input_id` _array_element))
    (bind _returnvalue (`KismetArrayLibrary.Array_Find` (`self.input_list`) _output_get))
    (if (>= _returnvalue 0)
      (set `local.local_input_index` _returnvalue)
      ;[1 1 1] if reseting defaults, replace the value of current input index by default one from stored local data.
      ; this is done to replace only the specific input that is going to reset, filtered by category or name.
      (if (`local.reset_defaults`)
        (`KismetArrayLibrary.Array_Set` (`self.input_data`) _local_input_index (`|GetArrayItem` (`local.local_default_data`) _local_input_index)))
      ;[1 1 1] load the input data for that input index that is currently in loop.
      (set `local.local_positive_keys` _positive_keys)
      (set `local.local_negative_keys` _negative_keys)
      (bind _output_get_2 (set `local.local_action_keys` _action_keys))
      (if (not (`KismetArrayLibrary.Array_IsValidIndex` _output_get_2))
        ;[1 1 1] clear and remove all axis mappings from input id first, to keep clean axis maps and prevent any duplicates.
        (bind (_arrayindex _arrayelement) (`/Engine/EditorBlueprintResources/StandardMacros.ReverseForEachLoop` (`InputSettings.GetAxisMappingByName` (`InputSettings.GetInputSettings`) (`local.local_input_id`)))
          (:`LoopBody`
            (`InputSettings.RemoveAxisMapping` (`InputSettings.GetInputSettings`) _arrayelement false))
          (:`Completed`
            ;[1 1 1] set axis map to engine, and check for local test arrays for invalid keys, and duplicates to prevent any duplication of input.
            ; first goes positive then negative keys, also check if negative key does not have positive keys,
            ; because axis key cannot have both same key mapped as positive and negative input,
            ; it is like gamepad stick should be mapped to axis only once to work properly.
            (for _array_element_2 (`local.local_positive_keys`)
              (bind _key (break `InputChord` _array_element_2))
              (if (not (`KismetArrayLibrary.Array_Contains` (`local.local_invalid_keys`) _key))
                (`InputSettings.AddAxisMapping` (`InputSettings.GetInputSettings`) (make `InputAxisKeyMapping` (`local.local_input_id`) _key) false)))
            (for _array_element_3 (`local.local_negative_keys`)
              (bind _key_2 (break `InputChord` _array_element_3))
              (if (`KismetArrayLibrary.Array_Contains` (`local.local_invalid_keys`) _key_2)
                _
                (elif (not (`KismetArrayLibrary.Array_Contains` (`local.local_positive_keys`) (make `InputChord` _key_2)))
                  (`InputSettings.AddAxisMapping` (`InputSettings.GetInputSettings`) (make `InputAxisKeyMapping` (`local.local_input_id`) _key_2 -1.0) false))))))
        (else
          ;[1 1 1] clear and remove all action mappings from input id first to keep clean action maps and prevent any duplicates.
          (bind (_arrayindex_2 _arrayelement_2) (`/Engine/EditorBlueprintResources/StandardMacros.ReverseForEachLoop` (`InputSettings.GetActionMappingByName` (`InputSettings.GetInputSettings`) (`local.local_input_id`)))
            (:`LoopBody`
              (`InputSettings.RemoveActionMapping` (`InputSettings.GetInputSettings`) _arrayelement_2 false))
            (:`Completed`
              ;[1 1 1] set action map to engine input and test check for local test array for invalid keys to prevent duplicates.
              (for _array_element_4 (`local.local_action_keys`)
                (bind (_key_3 _bshift _bctrl _balt _bcmd) (break `InputChord` _array_element_4))
                (if (not (`KismetArrayLibrary.Array_Contains` (`local.local_invalid_keys`) _key_3))
                  (`InputSettings.AddActionMapping` (`InputSettings.GetInputSettings`) (make `InputActionKeyMapping` (`local.local_input_id`) _key_3 _bshift _bctrl _balt _bcmd) false)))))))))
  ;[1 1 1] finalization, force rebuild keymaps after finish, and save key mappings input to engine and to custom save data if needed.
  (`InputSettings.ForceRebuildKeymaps` (`InputSettings.GetInputSettings`))
  (if (`local.save_inputs`)
    (`InputSettings.SaveKeyMappings` (`InputSettings.GetInputSettings`))
    (`self.save_input`)))

(fn `convert_action_keys`
  (params (action_key :type Name) (action_data :type "Array of Name"))
  (returns (input_chord :type "InputChord Structure"))
  ;[1 1 1] convert action keys from datatable data to input chord data.
  (bind _found_key (`self.get_key_by_id` action_key "AnyKey"))
  (return (make `InputChord` _found_key (>= (`KismetArrayLibrary.Array_Find` action_data "shift") 0) (>= (`KismetArrayLibrary.Array_Find` action_data "ctrl") 0) (>= (`KismetArrayLibrary.Array_Find` action_data "alt") 0) (>= (`KismetArrayLibrary.Array_Find` action_data "cmd") 0))))

(fn `convert_axis_keys`
  (params (data_axis :type "Array of Key Structure"))
  (returns (positive_chord :type "InputChord Structure") (negative_chord :type "InputChord Structure"))
  (locals (local_keys :type "Array of Key Structure") (local_positive :type "InputChord Structure") (local_negative :type "InputChord Structure"))
  (bind _local_keys (`local.local_keys`))
  (bind _local_keys_2 (`local.local_keys`))
  ;[1 1 1] convert axis keys from datatable data, to input chord data.
  (set `local.local_keys` data_axis)
  (`|ExecutionSequence`
    (:`then_0`
      (if (`KismetArrayLibrary.Array_IsValidIndex` _local_keys)
        (set `local.local_positive` (make `InputChord` (`|GetArrayItem` _local_keys)))))
    (:`then_1`
      (if (`KismetArrayLibrary.Array_IsValidIndex` _local_keys_2 1)
        (set `local.local_negative` (make `InputChord` (`|GetArrayItem` _local_keys_2 1)))))
    (:`then_2`
      (return (`local.local_positive`) (`local.local_negative`)))))

(fn `create_keys_data`
  ;[1 1 1] create all the keys list and keys data, its a meta-data for all the input that does exist in ue4,
  ; the list can be updated in datatable, if there are any new key input added for new devices, by new versions of engine.
  (`KismetArrayLibrary.Array_Clear` (`self.keys_list`))
  (`KismetArrayLibrary.Array_Clear` (`self.keys_data`))
  (bind _outrownames (`DataTableFunctionLibrary.GetDataTableRowNames` "/Game/MSL_Toolkit/settings_system/common/input_keys_data.input_keys_data"))
  (bind _output_get (set `self.keys_list` _outrownames))
  (for _array_element _output_get
    (bind _returnvalue (`|GetDataTableRow` "/Game/MSL_Toolkit/settings_system/common/input_keys_data.input_keys_data" _array_element)
      (:`then`
        (`KismetArrayLibrary.Array_Add` (`self.keys_data`) (`.key_2_D7019B844F66171D54D45E9936B46259` (break `/Game/MSL_Toolkit/settings_system/structs/s_input_key` _returnvalue)))))))

(fn `get_input_data`
  (params (input_id :type Name) (key_index :type Integer))
  (returns (input_data :type "/Game/MSL_Toolkit/settings_system/structs/s_input_data Structure") (positive_chord :type "InputChord Structure") (negative_chord :type "InputChord Structure") (positive_name :type Name) (negative_name :type Name) (input_category :type Name) (is_axis :type Boolean) (is_trigger :type Boolean))
  (locals (local_input_id :type Name) (local_input :type "/Game/MSL_Toolkit/settings_system/structs/s_input_data Structure") (local_input_index :type Integer) (local_pos_name :type Name) (local_neg_name :type Name) (local_category :type Name) (local_axis :type Boolean) (local_trigger :type Boolean))
  (bind _local_input_index (`local.local_input_index`))
  (bind (_positive_keys _negative_keys _action_keys) (break `/Game/MSL_Toolkit/settings_system/structs/s_input_data` (`local.local_input`)))
  (bind _returnvalue (`KismetArrayLibrary.Array_Find` (`self.input_list`) (`local.local_input_id`)))
  (bind _output (`|GetArrayItem` _action_keys _local_input_index))
  ;[1 1 1] get whole input data from current input list by specific input ID and key index.
  (set `local.local_input_id` input_id)
  (set `local.local_input_index` key_index)
  (if (>= _returnvalue 0)
    (set `local.local_input` (`|GetArrayItem` (`self.input_data`) _returnvalue))
    (`|ExecutionSequence`
      (:`then_0`
        (bind _returnvalue_2 (`|GetDataTableRow` "/Game/MSL_Toolkit/settings_system/common/input_default_axis.input_default_axis" (`local.local_input_id`))
          (:`then`
            (bind (_visual_positive_name _visual_negative_name _axis_pc _axis_gamepad _is_trigger _input_category) (break `/Game/MSL_Toolkit/settings_system/structs/s_input_axis` _returnvalue_2))
            (set `local.local_pos_name` _visual_positive_name)
            (set `local.local_neg_name` _visual_negative_name)
            (set `local.local_category` _input_category)
            (set `local.local_axis` true)
            (set `local.local_trigger` _is_trigger))
          (:`RowNotFound`
            (bind _returnvalue_3 (`|GetDataTableRow` "/Game/MSL_Toolkit/settings_system/common/input_default_action.input_default_action" (`local.local_input_id`))
              (:`then`
                (bind (_visual_action_name _action_pc _action_gamepad _input_category_2) (break `/Game/MSL_Toolkit/settings_system/structs/s_input_action` _returnvalue_3))
                (set `local.local_pos_name` _visual_action_name)
                (set `local.local_neg_name` _visual_action_name)
                (set `local.local_category` _input_category_2)
                (set `local.local_axis` false)
                (set `local.local_trigger` false))))))
      (:`then_1`
        (if (`local.local_axis`)
          (return (`local.local_input`) (`|GetArrayItem` _positive_keys _local_input_index) (`|GetArrayItem` _negative_keys _local_input_index) (`local.local_pos_name`) (`local.local_neg_name`) (`local.local_category`) (`local.local_axis`) (`local.local_trigger`))
          (else
            (return (`local.local_input`) _output _output (`local.local_pos_name`) (`local.local_neg_name`) (`local.local_category`) (`local.local_axis`) (`local.local_trigger`))))))
    (else
      (return (struct) (struct) (struct) "None" "None" "None" false false))))

(fn `get_inputs_by_category`
  (params (input_category :type Name) (all_categories :type Boolean))
  (returns (input_list :type "Array of Name"))
  (locals (local_array :type "Array of Name") (local_category :type Name) (local_name :type Name))
  ;[1 1 1] get all input names by specific category name, or from all categories by boolean.
  (set `local.local_category` input_category)
  (for _array_element (`self.input_list`)
    (bind _output_get (set `local.local_name` _array_element))
    (bind (_input_data _positive_chord _negative_chord _positive_name _negative_name _input_category) (`self.get_input_data` _output_get))
    (if (`local.all_categories`)
      (`KismetArrayLibrary.Array_Add` (`local.local_array`) (`local.local_name`) :!label _label)
      (elif (== _input_category (`local.local_category`))
        (goto _label))))
  (return (`local.local_array`)))

(fn `get_key_binds`
  (params (input_chord :type "InputChord Structure") (input_category :type Name))
  (returns (found_inputs :type "Array of Name") (found_positive :type "Array of Boolean") (found_keys :type "Array of Integer"))
  (locals (local_input_chord :type "InputChord Structure") (local_input_category :type Name) (local_input_id :type Name) (local_found_id :type "Array of Name") (local_found_positive :type "Array of Boolean") (local_found_index :type "Array of Integer") (local_positive :type "Array of InputChord Structure") (local_negative :type "Array of InputChord Structure") (local_action :type "Array of InputChord Structure") (local_key_index :type Integer))
  ;[1 1 1] get key bindings, so this function basically finds the same bindings within the specified category, to filter the duplicates.
  ; like you have key W binded in category general, if you are trying to bind W second time in the same category,
  ; you can check if there is key that using that to prevent duplicate binds.
  (set `local.local_input_chord` input_chord)
  (set `local.local_input_category` input_category)
  (for (_array_element _array_index) (`self.input_data`)
    (set `local.local_input_id` (`|GetArrayItem` (`self.input_list`) _array_index))
    (bind (_positive_keys _negative_keys _action_keys) (break `/Game/MSL_Toolkit/settings_system/structs/s_input_data` _array_element))
    (set `local.local_positive` _positive_keys)
    (set `local.local_negative` _negative_keys)
    (set `local.local_action` _action_keys)
    (bind (_input_data _positive_chord _negative_chord _positive_name _negative_name _input_category _is_axis) (`self.get_input_data` (`local.local_input_id`)))
    (if (== _input_category (`local.local_input_category`))
      (if _is_axis
        (for (_array_element_2 _array_index_2) (`local.local_positive`)
          (if (== _array_element_2 (`local.local_input_chord`))
            (set `local.local_key_index` _array_index_2)
            (`KismetArrayLibrary.Array_Add` (`local.local_found_id`) (`local.local_input_id`))
            (`KismetArrayLibrary.Array_Add` (`local.local_found_positive`) true)
            (`KismetArrayLibrary.Array_Add` (`local.local_found_index`) (`local.local_key_index`))))
        (for (_array_element_3 _array_index_3) (`local.local_negative`)
          (if (== _array_element_3 (`local.local_input_chord`))
            (set `local.local_key_index` _array_index_3)
            (`KismetArrayLibrary.Array_Add` (`local.local_found_id`) (`local.local_input_id`))
            (`KismetArrayLibrary.Array_Add` (`local.local_found_positive`))
            (`KismetArrayLibrary.Array_Add` (`local.local_found_index`) (`local.local_key_index`))))
        (else
          (for (_array_element_4 _array_index_4) (`local.local_action`)
            (if (== _array_element_4 (`local.local_input_chord`))
              (set `local.local_key_index` _array_index_4)
              (`KismetArrayLibrary.Array_Add` (`local.local_found_id`) (`local.local_input_id`))
              (`KismetArrayLibrary.Array_Add` (`local.local_found_positive`))
              (`KismetArrayLibrary.Array_Add` (`local.local_found_index`) (`local.local_key_index`))))))))
  (return (`local.local_found_id`) (`local.local_found_positive`) (`local.local_found_index`)))

(fn `get_key_by_id`
  (params (id_to_key :type Name) (key_to_id :type "Key Structure"))
  (returns (found_key :type "Key Structure") (found_id :type Name))
  (locals (local_empty :type "Key Structure" :default "None"))
  (bind _local_empty (`local.local_empty`))
  (bind _returnvalue (`KismetArrayLibrary.Array_Find` (`self.keys_list`) id_to_key))
  (bind _returnvalue_2 (`KismetArrayLibrary.Array_Find` (`self.keys_data`) key_to_id))
  (bind _returnvalue_3 (>= _returnvalue_2 0))
  (bind _output (`|GetArrayItem` (`self.keys_list`) _returnvalue_2))
  ;[1 1 1] find specific key by its ID from data key list, or specific ID from key data itself.
  ; can return both values at once.
  (if (>= _returnvalue 0)
    (if _returnvalue_3
      (return (`|GetArrayItem` (`self.keys_data`) _returnvalue) _output)
      (else
        _)))
  (if _returnvalue_3
    (return _local_empty _output)
    (else
      (return _local_empty "None"))))

(fn `get_key_visual_data`
  (params (key :type "Key Structure"))
  (returns (localized_name :type Text) (platform_icon :type "Texture2D Object Reference"))
  (locals (local_key_id :type Name) (local_name :type Text) (local_icon :type "Texture2D Object Reference") (local_id :type Name))
  (bind (_is_valid _from_data _line_text) (`/Game/MSL_Toolkit/localization_system/blueprints/bp_msl_localization_actor.get_text_localization` (`/Game/MSL_Toolkit/initial_system/msl_function_library.msl_get_localization_reference`) "keys" (`local.local_key_id`)))
  ;[1 1 1] find keys visual statement from datatable with visual key information, text/icon and etc.
  (bind (_found_key _found_id) (`self.get_key_by_id` "None" key))
  (set `local.local_key_id` _found_id)
  (bind _returnvalue (`|GetDataTableRow` "/Game/MSL_Toolkit/settings_system/common/input_keys_data.input_keys_data" (`local.local_key_id`))
    (:`then`
      (if _from_data
        (set `local.local_name` _line_text)
        (else
          (bind (_key _ps_icon _xb_icon _pc_icon) (break `/Game/MSL_Toolkit/settings_system/structs/s_input_key` _returnvalue))
          (set `local.local_name` (`KismetInputLibrary.Key_GetDisplayName` _key))))
      (if (`KismetInputLibrary.Key_IsGamepadKey` _key)
        (if (`self.ps4_icons`)
          (set `local.local_icon` _ps_icon)
          (else
            (set `local.local_icon` _xb_icon)))
        (else
          (set `local.local_icon` _pc_icon)))
      (return (`local.local_name`) (`local.local_icon`)))
    (:`RowNotFound`
      (return "UNKNOWN KEY" null))))

(fn `load_input`
  (params (load_defaults :type Boolean))
  (returns (input_list :type "Array of Name") (input_data :type "Array of /Game/MSL_Toolkit/settings_system/structs/s_input_data Structure") (loaded_defaults :type Boolean))
  (locals (local_default_input :type "Array of /Game/MSL_Toolkit/settings_system/structs/s_input_data Structure") (local_input_list :type "Array of Name") (local_axis_list :type "Array of Name") (local_action_list :type "Array of Name") (local_savefile :type Boolean :default false) (local_saved_input :type "Array of /Game/MSL_Toolkit/settings_system/structs/s_input_data Structure"))
  ;[1 1 1] load input logic, a complex function to build input list,
  ; and cleanly load defaults or saved data without any issues.
  (bind _returnvalue (`GameplayStatics.DoesSaveGameExist` (`self.save_settings_name`) (`self.save_user_index`)))
  (set `local.local_savefile` (and _returnvalue (not load_defaults)))
  (`|ExecutionSequence`
    (:`then_0`
      ;[1 1 1] first check if we are trying to load save file if it exist, then store the saved keybindings to local variable.
      (if (`local.local_savefile`)
        (bind _returnvalue_2 (`GameplayStatics.LoadGameFromSlot` (`self.save_settings_name`) (`self.save_user_index`)))
        (bind _asobject_input_save (cast `/Game/MSL_Toolkit/settings_system/blueprints/object_input_save` _returnvalue_2))
        (set `local.local_saved_input` (`/Game/MSL_Toolkit/settings_system/blueprints/object_input_save.keybindings_save` _asobject_input_save))))
    (:`then_1`
      ;[1 1 1] then we load all axis and action data, from datatables,
      ; all the input list should be appended, axis first then action, to build one big list of inputs.
      (bind _outrownames (`DataTableFunctionLibrary.GetDataTableRowNames` "/Game/MSL_Toolkit/settings_system/common/input_default_axis.input_default_axis"))
      (bind _output_get (set `local.local_axis_list` _outrownames))
      (`KismetArrayLibrary.Array_Append` (`local.local_input_list`) _output_get)
      (bind _outrownames_2 (`DataTableFunctionLibrary.GetDataTableRowNames` "/Game/MSL_Toolkit/settings_system/common/input_default_action.input_default_action"))
      (bind _output_get_2 (set `local.local_action_list` _outrownames_2))
      (`KismetArrayLibrary.Array_Append` (`local.local_input_list`) _output_get_2)
      ;[1 1 1] then we rebuild the input datatable data of names by converting it to actual input variable chords,
      ; first for all axis then for all actions.
      ; so basically we just convert text data to engine variable data.
      (for _array_element (`local.local_axis_list`)
        (bind _returnvalue_3 (`|GetDataTableRow` "/Game/MSL_Toolkit/settings_system/common/input_default_axis.input_default_axis" _array_element)
          (:`then`
            (bind (_visual_positive_name _visual_negative_name _axis_pc _axis_gamepad _is_trigger _input_category) (break `/Game/MSL_Toolkit/settings_system/structs/s_input_axis` _returnvalue_3))
            (`KismetArrayLibrary.Array_AddUnique` (`self.input_category`) _input_category)
            (bind (_positive_chord _negative_chord) (`self.convert_axis_keys` _axis_pc))
            (bind (_positive_chord_2 _negative_chord_2) (`self.convert_axis_keys` _axis_gamepad))
            (`KismetArrayLibrary.Array_Add` (`local.local_default_input`) (make `/Game/MSL_Toolkit/settings_system/structs/s_input_data` :`positive_keys` (`|MakeArray` _positive_chord _positive_chord_2) :`negative_keys` (`|MakeArray` _negative_chord _negative_chord_2))))))
      (for _array_element_2 (`local.local_action_list`)
        (bind _returnvalue_4 (`|GetDataTableRow` "/Game/MSL_Toolkit/settings_system/common/input_default_action.input_default_action" _array_element_2)
          (:`then`
            (bind (_visual_action_name _action_pc _action_gamepad _input_category_2) (break `/Game/MSL_Toolkit/settings_system/structs/s_input_action` _returnvalue_4))
            (`KismetArrayLibrary.Array_AddUnique` (`self.input_category`) _input_category_2)
            (`KismetArrayLibrary.Array_Add` (`local.local_default_input`) (make `/Game/MSL_Toolkit/settings_system/structs/s_input_data` :`action_keys` (`|MakeArray` (make `InputChord` _action_pc) (make `InputChord` _action_gamepad)))))))
      ;[1 1 1] finally checking if save file needs to be load, if it so then we should compare the saved input data with default input data,
      ; if they are not equal then new inputs is added to default ones, this means that game is patched or something else,
      ; if this happens we just return the default data, but if they are equal we will return save file data, if we don't need to load save file we return default input.
      (if (`local.local_savefile`)
        (if (== (`KismetArrayLibrary.Array_Length` (`local.local_default_input`)) (`KismetArrayLibrary.Array_Length` (`local.local_saved_input`)))
          (return (`local.local_input_list`) (`local.local_saved_input`) false)
          (else
            (`GameplayStatics.DeleteGameInSlot` (`self.save_settings_name`) (`self.save_user_index`)) ; delete settings save, if its not valid.
          )))
      (return (`local.local_input_list`) (`local.local_default_input`) true))))

(fn `rebind_input`
  (params (both_axis :type Boolean) (positive_axis :type Boolean) (key_index :type Integer) (input_id :type Name) (input_chord :type "InputChord Structure"))
  (locals (local_both_axis :type Boolean) (local_positive :type Boolean) (local_key_index :type Integer) (local_input_id :type Name) (local_input_chord :type "InputChord Structure") (local_axis :type Boolean) (local_category :type Name))
  ;[1 1 1] rebinds the current input key to specific one that is needed, with filtering and handling the duplicates and removing any conflicts.
  ; should be used generally to rebind any input key.
  (set `local.local_both_axis` both_axis)
  (set `local.local_positive` positive_axis)
  (set `local.local_key_index` key_index)
  (set `local.local_input_id` input_id)
  (set `local.local_input_chord` input_chord)
  (if (>= (`KismetArrayLibrary.Array_Find` (`self.input_list`) (`local.local_input_id`)) 0)
    (bind (_input_data _positive_chord _negative_chord _positive_name _negative_name _input_category _is_axis) (`self.get_input_data` (`local.local_input_id`)))
    (set `local.local_category` _input_category)
    (set `local.local_axis` _is_axis)
    ;[1 1 1] remove duplicate/conflicted bindings by category, same keys from same input category
    ; will be set to none, before settings the new key
    (bind (_found_inputs _found_positive _found_keys) (`self.get_key_binds` (`local.local_input_chord`) (`local.local_category`)))
    (bind (_arrayindex _arrayelement) (`/Engine/EditorBlueprintResources/StandardMacros.ReverseForEachLoop` _found_inputs)
      (:`LoopBody`
        (if (and (== (`local.local_input_id`) _arrayelement) (`KismetInputLibrary.Key_IsFloatAxis` (`.Key` (break `InputChord` (`local.local_input_chord`)))))
          (bind _output (`|GetArrayItem` _found_keys _arrayindex))
          (if (not (== _output (`local.local_key_index`)))
            (`self.set_bind` _arrayelement (`|GetArrayItem` _found_positive _arrayindex) _output :!label _label))
          (else
            (goto _label))))
      (:`Completed`
        (if (`local.local_axis`)
          (if (`local.local_both_axis`)
            ;[1 1 1] both axis is optional, and it does that like if you use left stick to bind look up and down,
            ; it will map both of those to left stick axis, so you don't need to map second one to same key.
            (`self.set_bind` (`local.local_input_id`) false (`local.local_key_index`) (`local.local_input_chord`))
            (`self.set_bind` (`local.local_input_id`) true (`local.local_key_index`) (`local.local_input_chord`))
            (else
              ;[1 1 1] sets positive and negative input separately for axis, should be used for most times.
              ; because most keys are not gamepad sticks those are not true axis keys,
              ; so they should be mapped separately to positive and negative axis.
              (`self.set_bind` (`local.local_input_id`) (`local.local_positive`) (`local.local_key_index`) (`local.local_input_chord`))))
          (else
            ;[1 1 1] if the input is not axis itself, it does map action.
            (`self.set_bind` (`local.local_input_id`) false (`local.local_key_index`) (`local.local_input_chord`))))))))

(fn `save_input`
  ;[1 1 1] save input data, to file, if it exist just load it and replace only input data and save it again.
  (bind _returnvalue (`GameplayStatics.DoesSaveGameExist` (`self.save_settings_name`) (`self.save_user_index`)))
  (if _returnvalue
    (bind _returnvalue_2 (`GameplayStatics.LoadGameFromSlot` (`self.save_settings_name`) (`self.save_user_index`)))
    (bind _asobject_input_save (cast `/Game/MSL_Toolkit/settings_system/blueprints/object_input_save` _returnvalue_2))
    (set `/Game/MSL_Toolkit/settings_system/blueprints/object_input_save.keybindings_save` (`self.input_data`) _asobject_input_save)
    (`GameplayStatics.SaveGameToSlot` _asobject_input_save (`self.save_settings_name`) (`self.save_user_index`))
    (else
      (bind _returnvalue_3 (`GameplayStatics.CreateSaveGameObject` "/Game/MSL_Toolkit/settings_system/blueprints/object_input_save.object_input_save_C"))
      (set `/Game/MSL_Toolkit/settings_system/blueprints/object_input_save.keybindings_save` (`self.input_data`) _returnvalue_3)
      (`GameplayStatics.SaveGameToSlot` _returnvalue_3 (`self.save_settings_name`) (`self.save_user_index`)))))

(fn `set_bind`
  (params (input_id :type Name) (positive_axis :type Boolean) (key_index :type Integer) (input_chord :type "InputChord Structure"))
  (locals (local_positive_axis :type Boolean) (local_input_id :type Name) (local_key_index :type Integer) (local_input_chord :type "InputChord Structure") (local_axis :type Boolean) (local_positive :type "Array of InputChord Structure") (local_negative :type "Array of InputChord Structure") (local_action :type "Array of InputChord Structure"))
  (bind _returnvalue (`KismetArrayLibrary.Array_Find` (`self.input_list`) (`local.local_input_id`)))
  (bind _output (`|GetArrayItem` (`self.input_data`) _returnvalue))
  (bind (_positive_keys _negative_keys _action_keys) (break `/Game/MSL_Toolkit/settings_system/structs/s_input_data` _output))
  ;[1 1 1] sets the actual bind to input id with the specific key and key index.
  ; should not be called directly, use "rebind_input" instead
  (set `local.local_input_id` input_id)
  (set `local.local_positive_axis` positive_axis)
  (set `local.local_key_index` key_index)
  (set `local.local_input_chord` input_chord)
  (if (>= _returnvalue 0)
    (set `local.local_positive` _positive_keys)
    (set `local.local_negative` _negative_keys)
    (bind _output_get (set `local.local_action` _action_keys))
    (if (not (`KismetArrayLibrary.Array_IsValidIndex` _output_get))
      (setmembers `InputChord` :`StructRef` (`local.local_input_chord`) :`bShift` false :`bCtrl` false :`bAlt` false :`bCmd` false)
      (if (`local.local_positive_axis`)
        (`KismetArrayLibrary.Array_Set` (`local.local_positive`) (`local.local_key_index`) (`local.local_input_chord`))
        (setmembers `/Game/MSL_Toolkit/settings_system/structs/s_input_data` :`StructRef` _output :`positive_keys` (`local.local_positive`))
        (else
          (`KismetArrayLibrary.Array_Set` (`local.local_negative`) (`local.local_key_index`) (`local.local_input_chord`))
          (setmembers `/Game/MSL_Toolkit/settings_system/structs/s_input_data` :`StructRef` _output :`negative_keys` (`local.local_negative`))))
      (else
        (`KismetArrayLibrary.Array_Set` (`local.local_action`) (`local.local_key_index`) (`local.local_input_chord`))
        (setmembers `/Game/MSL_Toolkit/settings_system/structs/s_input_data` :`StructRef` _output :`action_keys` (`local.local_action`))))))

(fn `UserConstructionScript`)