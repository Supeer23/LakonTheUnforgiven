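; Dialogue-system proxy that stands in for a widget, with components that preview its scale.
; The construction script calls the parent's, then remaps WidgetScale to a uniform world scale on WScale.
; Custom proxy init destroys the WScale, WBack and WFront dummy components.
; Custom proxy tick writes WidgetScale to the "widget_scale" float variable.
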(event `self.custom_proxy_init`
  ;[1 1 1] Beginplay for dummy widget
  ; is here.
  (`ActorComponent.K2_DestroyComponent` (`self.w_scale`))
  (`ActorComponent.K2_DestroyComponent` (`self.w_back`))
  (`ActorComponent.K2_DestroyComponent` (`self.w_front`)))

(event `self.custom_proxy_tick`
  (params (delta_seconds :type "Float (single-precision)"))
  ;[1 1 1] Beginplay for dummy widget
  ; is here.
  (`self.set_float_var` "widget_scale" (`self.widget_scale`)))

(fn `update_widget_scale`
  ;[1 1 1] Update the widget scale.
  (`SceneComponent.SetWorldScale3D` (`self.w_scale`) (`KismetMathLibrary.Conv_DoubleToVector` (`KismetMathLibrary.MapRangeUnclamped` (`self.widget_scale`) 0.0 1.0 0.0 0.1))))

(fn `UserConstructionScript`
  (`parent.UserConstructionScript`)
  (`self.update_widget_scale`))