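; Generic quest marker Blueprint that shows a quest objective as an icon through the DLG map system.
; Its init event stores the quest actor, objective and sub-objective, then asks the owning quest component whether that quest is active.
; The active quest's index selects a red, green or blue icon tint, with white when none is found.
; It then updates the map component's registration; the icon-type switch has no visible branches.
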(event `init_quest_icon`
  (params (quest_actor :type "/Game/DLG_Tree/dqst_system/blueprints/bp_quest_actor Object Reference") (objective_id :type Name) (sub_objective :type Boolean) (icon_type :type "/Game/DLG_Tree/dqst_system/structs/09_enums/enum_quest_icon Enum" :default "NewEnumerator0"))
  (bind _quest_actor (`self.quest_actor`))
  ;[1 1 1] This is generic quest marker for icons.
  ; Beginplay is here.
  (set `self.quest_actor` quest_actor)
  (set `self.objective_id` objective_id)
  (set `self.sub_objective` sub_objective)
  (`|ExecutionSequence`
    (:`then_0`
      (switch `/Game/DLG_Tree/dqst_system/structs/09_enums/enum_quest_icon` icon_type))
    (:`then_1`
      (bind (_is_valid _found_index) (`/Game/DLG_Tree/dqst_system/blueprints/bp_quest_component.get_quest_active` (`/Game/DLG_Tree/dqst_system/blueprints/bp_quest_actor.owning_quest_component` _quest_actor) (`/Game/DLG_Tree/dqst_system/blueprints/bp_quest_actor.quest_unique_id` _quest_actor)))
      (if _is_valid
        (switch `int` _found_index
          (:`0`
            (setmembers `/Game/DLG_Tree/dmap_system/structs/s_dlg_icon_data` :`StructRef` (`/Game/DLG_Tree/dmap_system/blueprints/bp_dlg_map_component.icon_info` (`self.bp_dlg_map_component`)) :`icon_color` (struct :`R` 1.0 :`G` 0.05 :`B` 0.05 :`A` 1.0)))
          (:`1`
            (setmembers `/Game/DLG_Tree/dmap_system/structs/s_dlg_icon_data` :`StructRef` (`/Game/DLG_Tree/dmap_system/blueprints/bp_dlg_map_component.icon_info` (`self.bp_dlg_map_component`)) :`icon_color` (struct :`R` 0.05 :`G` 1.0 :`B` 0.244333 :`A` 1.0)))
          (:`2`
            (setmembers `/Game/DLG_Tree/dmap_system/structs/s_dlg_icon_data` :`StructRef` (`/Game/DLG_Tree/dmap_system/blueprints/bp_dlg_map_component.icon_info` (`self.bp_dlg_map_component`)) :`icon_color` (struct :`R` 0.05 :`G` 0.294997 :`B` 1.0 :`A` 1.0))))
        (else
          (setmembers `/Game/DLG_Tree/dmap_system/structs/s_dlg_icon_data` :`StructRef` (`/Game/DLG_Tree/dmap_system/blueprints/bp_dlg_map_component.icon_info` (`self.bp_dlg_map_component`)) :`icon_color` (struct :`R` 1.0 :`G` 1.0 :`B` 1.0 :`A` 1.0)))))
    (:`then_2`
      (`/Game/DLG_Tree/dmap_system/blueprints/bp_dlg_map_component.update_register` (`self.bp_dlg_map_component`) true))))

(fn `UserConstructionScript`)