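; Notification component that queues on-screen notification widgets and shows them in a limited set of active slots.
; SpawnNotification creates a given or default slot widget with two texts, queues it, and runs CheckNotification.
; CheckNotification moves queued widgets into free slots and starts them, optionally holding the queue after the last slot fills until all clear.
; ReturnNotification frees a finished widget's slot and rechecks the queue.
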(event `self.ReceiveBeginPlay`
  ;[1 1 1] Notification component,
  ; Beginplay is here.
  (`KismetArrayLibrary.Array_Resize` (`self.active_notifications`) (`self.max_notifications`)))

(fn `check_notification`
  (locals (local_exist :type Boolean) (local_index :type Integer :default 0) (local_target :type "Object Object Reference"))
  ;[1 1 1] Check notification logic,
  ; if hit last select empty, or wait until they clear.
  (for _ (range (+ (`self.max_notifications`) 1))
    (if (`KismetArrayLibrary.Array_IsValidIndex` (`self.notifications_queue`))
      (set `local.local_target` (`|GetArrayItem` (`self.notifications_queue`)))
      (set `local.local_index` (`KismetArrayLibrary.Array_Find` (`self.active_notifications`)))
      (if (>= (`local.local_index`) 0)
        (if (`self.is_hit_last`)
          (if (`self.wait_until_empty`)
            (for _array_element (`self.active_notifications`)
              (`/Engine/EditorBlueprintResources/StandardMacros.IsValid` _array_element
                (:`Is Valid`
                  (set `local.local_exist` true)
                  (break))))))
        (if (not (`local.local_exist`))
          (set `self.is_hit_last` (== (`local.local_index`) (- (`self.max_notifications`) 1)))
          (`KismetArrayLibrary.Array_Remove` (`self.notifications_queue`))
          (`KismetArrayLibrary.Array_Set` (`self.active_notifications`) (`local.local_index`) (`local.local_target`))
          (bind _asw_01_notification_parent (cast `/Game/DLG_Tree/dqst_system/widgets/notify/w_01_notification_parent` (`local.local_target`)))
          (`/Game/DLG_Tree/dqst_system/widgets/notify/w_01_notification_parent.start_notification` _asw_01_notification_parent (`local.local_index`)))))))

(fn `return_notification`
  (params (active_index :type Integer))
  ;[1 1 1] Return notification logic,
  ; on finished.
  (`KismetArrayLibrary.Array_Set` (`self.active_notifications`) active_index)
  (`self.check_notification`))

(fn `spawn_notification`
  (params (notification_class :type "/Game/DLG_Tree/dqst_system/widgets/notify/w_01_notification_parent Class Reference") (text1 :type Text) (text2 :type Text))
  (returns (notify_widget :type "/Game/DLG_Tree/dqst_system/widgets/notify/w_01_notification_parent Object Reference"))
  (locals (local_class :type "/Game/DLG_Tree/dqst_system/widgets/notify/w_01_notification_parent Class Reference"))
  ;[1 1 1] Spawn notification logic.
  (if (`KismetSystemLibrary.IsValidClass` notification_class)
    (set `local.local_class` notification_class)
    (else
      (set `local.local_class` "/Game/DLG_Tree/dqst_system/widgets/notify/w_02_notification_slot.w_02_notification_slot_C")))
  (bind _returnvalue (`|CreateWidget` (`local.local_class`)))
  (bind _returnvalue_2 (`KismetArrayLibrary.Array_Add` (`self.notifications_queue`) _returnvalue))
  (`/Game/DLG_Tree/dqst_system/widgets/notify/w_01_notification_parent.add_notification` _returnvalue self _returnvalue_2)
  (`/Game/DLG_Tree/dqst_system/widgets/notify/w_01_notification_parent.custom_notify_info` _returnvalue text1 text2)
  (`self.check_notification`)
  (return _returnvalue))