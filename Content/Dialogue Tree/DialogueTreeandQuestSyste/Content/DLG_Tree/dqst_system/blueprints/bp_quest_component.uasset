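; Quest manager component that spawns one quest actor per unique ID and relays its result, objective and event updates through dispatchers.
; It tracks an active-quest list with a size limit and optional removal of the oldest, plus a timestamped history.
; Saves are keyed by the owner's identifier, with history packed into option strings.
; Loading respawns quests without initialization, then restores status, objectives and active state.
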(event `self.ReceiveBeginPlay`
  ;[1 1 1] Quest component,
  ; beginplay is here.
)

(event `quest_call_result`
  (params (qst_actor :type "/Game/DLG_Tree/dqst_system/blueprints/bp_quest_actor Object Reference") (qst_result :type "/Game/DLG_Tree/dqst_system/structs/09_enums/enum_quest_result Enum" :default "NewEnumerator2"))
  ;[1 1 1] Basic Data events.
  (`self.ed_qst_result` qst_actor qst_result))

(event `init_player`
  ;[1 1 1] Quest component,
  ; beginplay is here.
  (bind (_is_valid _quest_widget) (`self.get_layout_widget`))
  (if _is_valid
    (`/Game/DLG_Tree/dqst_system/widgets/base/w_01_quest_layout.init_player` _quest_widget self)))

(event `quest_call_obj_added`
  (params (qst_actor :type "/Game/DLG_Tree/dqst_system/blueprints/bp_quest_actor Object Reference") (objective_id :type Name) (is_removed :type Boolean))
  ;[1 1 1] Basic Data events.
  (`self.ed_qst_obj_added` qst_actor objective_id is_removed))

(event `self.ReceiveEndPlay`
  (params (EndPlayReason :type "EEndPlayReason Enum" :default "Destroyed"))
  ;[1 1 1] Quest component,
  ; beginplay is here.
  (`self.destroy_quests`))

(event `quest_call_obj_update`
  (params (qst_actor :type "/Game/DLG_Tree/dqst_system/blueprints/bp_quest_actor Object Reference") (objective_id :type Name) (objective_result :type "/Game/DLG_Tree/dqst_system/structs/09_enums/enum_quest_result Enum" :default "NewEnumerator2"))
  ;[1 1 1] Basic Data events.
  (`self.ed_qst_obj_update` qst_actor objective_id objective_result))

(event `self.ReceiveTick`
  (params (DeltaSeconds :type "Float (single-precision)"))
  ;[1 1 1] Quest component,
  ; beginplay is here.
)

(event `quest_call_sub_obj_update`
  (params (qst_actor :type "/Game/DLG_Tree/dqst_system/blueprints/bp_quest_actor Object Reference") (objective_id :type Name) (sub_objective_id :type Name) (objective_current :type Integer) (objective_target :type Integer) (objective_result :type "/Game/DLG_Tree/dqst_system/structs/09_enums/enum_quest_result Enum" :default "NewEnumerator2"))
  ;[1 1 1] Basic Data events.
  (`self.ed_qst_sub_obj_update` qst_actor objective_id sub_objective_id objective_current objective_target objective_result))

(event `quest_call_event`
  (params (qst_actor :type "/Game/DLG_Tree/dqst_system/blueprints/bp_quest_actor Object Reference") (quest_event :type "/Game/DLG_Tree/dqst_system/structs/01_quest/s_quest_event Structure"))
  ;[1 1 1] Basic Data events.
  (`self.ed_qst_event` qst_actor quest_event))

(fn `add_quest`
  (params (quest_unique_id :type Name) (quest_data_id :type Name))
  (returns (is_valid :type Boolean) (is_spawned :type Boolean) (quest_actor :type "/Game/DLG_Tree/dqst_system/blueprints/bp_quest_actor Object Reference"))
  (locals (local_unique_id :type Name) (local_actor :type "/Game/DLG_Tree/dqst_system/blueprints/bp_quest_actor Object Reference") (local_quest_data :type Name))
  ;[1 1 1] Spawn and add to manager.
  (set `local.local_unique_id` quest_unique_id)
  (set `local.local_quest_data` quest_data_id)
  (if (!= (`local.local_unique_id`) "None")
    (bind (_is_valid _found_index _quest_actor) (`self.get_quest` (`local.local_unique_id`)))
    (if _is_valid
      (set `local.local_actor` _quest_actor)
      (return true false (`local.local_actor`))
      (else
        (bind _returnvalue (`|SpawnActorFromClass` "/Game/DLG_Tree/dqst_system/blueprints/bp_quest_actor.bp_quest_actor_C" (`KismetMathLibrary.MakeTransform` (0.0 0.0 0.0)) "AlwaysSpawn" "OverrideRootScale" null null))
        (set `local.local_actor` _returnvalue)
        (`|ExecutionSequence`
          (:`then_0`
            (`KismetArrayLibrary.Array_Add` (`self.quest_list`) (`local.local_unique_id`))
            (`KismetArrayLibrary.Array_Add` (`self.quest_actors`) (`local.local_actor`)))
          (:`then_1`
            (bind (_is_valid_2 _found_index_2) (`self.get_quest_history` (`local.local_unique_id`)))
            (if _is_valid_2
              (`KismetArrayLibrary.Array_Set` (`self.quest_history_time`) _found_index_2 (`KismetMathLibrary.Now`))
              (else
                (`KismetArrayLibrary.Array_Add` (`self.quest_history_list`) (`local.local_unique_id`))
                (`KismetArrayLibrary.Array_Add` (`self.quest_history_time`) (`KismetMathLibrary.Now`)))))
          (:`then_2`
            (`/Game/DLG_Tree/dqst_system/blueprints/bp_quest_actor.init_quest_data` (`local.local_actor`) (`local.local_unique_id`) (`local.local_quest_data`) self false)
            (`self.ed_qst_added` (`local.local_actor`))
            (return true true (`local.local_actor`))))))
    (else
      (return false false null))))

(fn `add_quest_loading`
  (params (quest_unique_id :type Name) (quest_data_id :type Name))
  (returns (is_valid :type Boolean) (is_spawned :type Boolean) (quest_actor :type "/Game/DLG_Tree/dqst_system/blueprints/bp_quest_actor Object Reference"))
  (locals (local_unique_id :type Name) (local_actor :type "/Game/DLG_Tree/dqst_system/blueprints/bp_quest_actor Object Reference") (local_quest_data :type Name))
  ;[1 1 1] Spawn and add to manager.
  (set `local.local_unique_id` quest_unique_id)
  (set `local.local_quest_data` quest_data_id)
  (if (!= (`local.local_unique_id`) "None")
    (bind (_is_valid _found_index _quest_actor) (`self.get_quest` (`local.local_unique_id`)))
    (if _is_valid
      (set `local.local_actor` _quest_actor)
      (return true false (`local.local_actor`))
      (else
        (bind _returnvalue (`|SpawnActorFromClass` "/Game/DLG_Tree/dqst_system/blueprints/bp_quest_actor.bp_quest_actor_C" (`KismetMathLibrary.MakeTransform` (0.0 0.0 0.0)) "AlwaysSpawn" "OverrideRootScale" null null))
        (set `local.local_actor` _returnvalue)
        (`|ExecutionSequence`
          (:`then_0`
            (`KismetArrayLibrary.Array_Add` (`self.quest_list`) (`local.local_unique_id`))
            (`KismetArrayLibrary.Array_Add` (`self.quest_actors`) (`local.local_actor`)))
          (:`then_1`
            (bind (_is_valid_2 _found_index_2) (`self.get_quest_history` (`local.local_unique_id`)))
            (if _is_valid_2
              (`KismetArrayLibrary.Array_Set` (`self.quest_history_time`) _found_index_2 (`KismetMathLibrary.Now`))
              (else
                (`KismetArrayLibrary.Array_Add` (`self.quest_history_list`) (`local.local_unique_id`))
                (`KismetArrayLibrary.Array_Add` (`self.quest_history_time`) (`KismetMathLibrary.Now`)))))
          (:`then_2`
            (`/Game/DLG_Tree/dqst_system/blueprints/bp_quest_actor.init_quest_data` (`local.local_actor`) (`local.local_unique_id`) (`local.local_quest_data`) self true)
            (`self.ed_qst_added` (`local.local_actor`))
            (return true true (`local.local_actor`))))))
    (else
      (return false false null))))

(fn `destroy_quests`
  ;[1 1 1] Clear quests.
  (bind (_arrayindex _arrayelement) (`/Engine/EditorBlueprintResources/StandardMacros.ReverseForEachLoop` (`self.quest_actors`))
    (:`LoopBody`
      (`/Engine/EditorBlueprintResources/StandardMacros.IsValid` _arrayelement
        (:`Is Valid`
          (`/Game/DLG_Tree/dqst_system/blueprints/bp_quest_actor.delayed_destroy` _arrayelement))))))

(fn `get_layout_widget`
  (returns (is_valid :type Boolean) (quest_widget :type "/Game/DLG_Tree/dqst_system/widgets/base/w_01_quest_layout Object Reference"))
  ;[1 1 1] Get widget layout.
  (bind _foundwidgets (`WidgetBlueprintLibrary.GetAllWidgetsOfClass` "/Game/DLG_Tree/dqst_system/widgets/base/w_01_quest_layout.w_01_quest_layout_C"))
  (bind _returnvalue (`KismetArrayLibrary.Array_LastIndex` _foundwidgets))
  (bind _returnvalue_2 (`KismetArrayLibrary.Array_IsValidIndex` _foundwidgets _returnvalue))
  (if _returnvalue_2
    (return _returnvalue_2 (`|GetArrayItem` _foundwidgets _returnvalue))
    (else
      (return false null))))

(fn `get_quest`
  (params (quest_unique_id :type Name))
  (returns (is_valid :type Boolean) (found_index :type Integer) (quest_actor :type "/Game/DLG_Tree/dqst_system/blueprints/bp_quest_actor Object Reference"))
  (bind _returnvalue (`KismetArrayLibrary.Array_Find` (`self.quest_list`) quest_unique_id))
  (bind _returnvalue_2 (>= _returnvalue 0))
  ;[1 1 1] Comment
  (if _returnvalue_2
    (return _returnvalue_2 _returnvalue (`|GetArrayItem` (`self.quest_actors`) _returnvalue))
    (else
      (return false 0 null))))

(fn `get_quest_active`
  (params (quest_unique_id :type Name))
  (returns (is_valid :type Boolean) (found_index :type Integer))
  (bind _returnvalue (`KismetArrayLibrary.Array_Find` (`self.active_quest`) quest_unique_id))
  (bind _returnvalue_2 (>= _returnvalue 0))
  ;[1 1 1] Get active quest by id.
  (if _returnvalue_2
    (return _returnvalue_2 _returnvalue)
    (else
      (return false 0))))

(fn `get_quest_history`
  (params (quest_unique_id :type Name))
  (returns (is_valid :type Boolean) (found_index :type Integer) (latest_time :type "DateTime Structure"))
  (bind _returnvalue (`KismetArrayLibrary.Array_Find` (`self.quest_history_list`) quest_unique_id))
  (bind _returnvalue_2 (>= _returnvalue 0))
  ;[1 1 1] Get quest history by ID and time.
  (if _returnvalue_2
    (return _returnvalue_2 _returnvalue (`|GetArrayItem` (`self.quest_history_time`) _returnvalue))
    (else
      (return false 0))))

(fn `quest_load_info`
  (locals (local_quest_list :type "Array of /Game/DLG_Tree/dqst_system/structs/05_savegame/s_quest_savegame Structure") (local_actor :type "/Game/DLG_Tree/dqst_system/blueprints/bp_quest_actor Object Reference"))
  (bind _local_quest_list (`local.local_quest_list`))
  ;[1 1 1] Dlg load all quests after save is loaded.
  (`self.destroy_quests`)
  (`|ExecutionSequence`
    (:`then_0`
      (bind (_is_valid _found_var_index _found_var_data) (`/Game/MSL_Toolkit/savegame_system/blueprints/bp_msl_savegame_actor.get_saved_var_info` (`/Game/MSL_Toolkit/initial_system/msl_function_library.msl_get_savegame_reference`) "base" "qst" "base" (`.actor_unique_id` (`/Game/MSL_Toolkit/savegame_system/blueprints/bp_msl_identifier_component.get_id` (`.identifier_reference` (`/Game/MSL_Toolkit/initial_system/msl_function_library.msl_get_identifier_component` (`self.GetOwner`))))) "qst_info" "None" true))
      (set `local.local_quest_list` (`.qst_var_25_4A79980A4C62E17060CE1AA006241243` (break `/Game/MSL_Toolkit/savegame_system/structs/var/s_save_var_data` _found_var_data)))
      (for _array_element (`local.local_quest_list`)
        (bind (_quest_active _quest_unique_id _quest_data_id _quest_status _quest_data _description_list _objective_list _objective_data) (break `/Game/DLG_Tree/dqst_system/structs/05_savegame/s_quest_savegame` _array_element))
        (bind (_is_valid_2 _is_spawned _quest_actor) (`self.add_quest_loading` _quest_unique_id _quest_data_id))
        (set `local.local_actor` _quest_actor)
        (`|ExecutionSequence`
          (:`then_0`
            (set `/Game/DLG_Tree/dqst_system/blueprints/bp_quest_actor.quest_status` _quest_status (`local.local_actor`))
            (set `/Game/DLG_Tree/dqst_system/blueprints/bp_quest_actor.quest_data` _quest_data (`local.local_actor`))
            (set `/Game/DLG_Tree/dqst_system/blueprints/bp_quest_actor.description_list` _description_list (`local.local_actor`)))
          (:`then_1`
            (set `/Game/DLG_Tree/dqst_system/blueprints/bp_quest_actor.objective_list` _objective_list (`local.local_actor`))
            (set `/Game/DLG_Tree/dqst_system/blueprints/bp_quest_actor.objective_data` _objective_data (`local.local_actor`)))))
      (for (_ _array_index) (`self.quest_actors`)
        (if (`KismetArrayLibrary.Array_IsValidIndex` _local_quest_list _array_index)
          (bind (_quest_active_2 _quest_unique_id_2) (break `/Game/DLG_Tree/dqst_system/structs/05_savegame/s_quest_savegame` (`|GetArrayItem` _local_quest_list _array_index)))
          (if _quest_active_2
            (`self.set_quest_active` _quest_unique_id_2)))))
    (:`then_1`
      (bind (_is_valid_3 _found_var_index_2 _found_var_data_2) (`/Game/MSL_Toolkit/savegame_system/blueprints/bp_msl_savegame_actor.get_saved_var_info` (`/Game/MSL_Toolkit/initial_system/msl_function_library.msl_get_savegame_reference`) "base" "qst" "base" (`.actor_unique_id` (`/Game/MSL_Toolkit/savegame_system/blueprints/bp_msl_identifier_component.get_id` (`.identifier_reference` (`/Game/MSL_Toolkit/initial_system/msl_function_library.msl_get_identifier_component` (`self.GetOwner`))))) "qst_history" "None" true))
      (for _array_element_2 (`.string_var_9_5CF9554843E46CD6C5F01EA7310CA938` (break `/Game/MSL_Toolkit/savegame_system/structs/var/s_save_var_data` _found_var_data_2))
        (`KismetArrayLibrary.Array_Add` (`self.quest_history_list`) (`KismetStringLibrary.Conv_StringToName` (`GameplayStatics.ParseOption` _array_element_2 "qstid")))
        (bind _returnvalue (`KismetStringLibrary.ParseIntoArray` (`GameplayStatics.ParseOption` _array_element_2 "qsttime") "*"))
        (`KismetArrayLibrary.Array_Add` (`self.quest_history_time`) (`KismetMathLibrary.MakeDateTime` (`KismetStringLibrary.Conv_StringToInt` (`|GetArrayItem` _returnvalue)) (`KismetStringLibrary.Conv_StringToInt` (`|GetArrayItem` _returnvalue 1)) (`KismetStringLibrary.Conv_StringToInt` (`|GetArrayItem` _returnvalue 2)) (`KismetStringLibrary.Conv_StringToInt` (`|GetArrayItem` _returnvalue 3)) (`KismetStringLibrary.Conv_StringToInt` (`|GetArrayItem` _returnvalue 4)) (`KismetStringLibrary.Conv_StringToInt` (`|GetArrayItem` _returnvalue 5)) (`KismetStringLibrary.Conv_StringToInt` (`|GetArrayItem` _returnvalue 6))))))))

(fn `quest_save_info`
  ;[1 1 1] Save quest info logic.
  (`/Game/MSL_Toolkit/savegame_system/blueprints/bp_msl_savegame_actor.remove_saved_var` (`/Game/MSL_Toolkit/initial_system/msl_function_library.msl_get_savegame_reference`) "base" "qst" "base" (`.actor_unique_id` (`/Game/MSL_Toolkit/savegame_system/blueprints/bp_msl_identifier_component.get_id` (`.identifier_reference` (`/Game/MSL_Toolkit/initial_system/msl_function_library.msl_get_identifier_component` (`self.GetOwner`))))) "None" "None" "branch" false true)
  (`|ExecutionSequence`
    (:`then_0`
      (for (_array_element _array_index) (`self.quest_actors`)
        (bind _quest_save (`/Game/DLG_Tree/dqst_system/blueprints/bp_quest_actor.get_save_data` _array_element))
        (`/Game/MSL_Toolkit/savegame_system/blueprints/bp_msl_savegame_actor.save_qst_var` (`/Game/MSL_Toolkit/initial_system/msl_function_library.msl_get_savegame_reference`) "base" "qst" "base" (`.actor_unique_id` (`/Game/MSL_Toolkit/savegame_system/blueprints/bp_msl_identifier_component.get_id` (`.identifier_reference` (`/Game/MSL_Toolkit/initial_system/msl_function_library.msl_get_identifier_component` (`self.GetOwner`))))) "qst_info" (`KismetStringLibrary.Conv_StringToName` (`KismetStringLibrary.Conv_IntToString` _array_index)) _quest_save false true)))
    (:`then_1`
      (for (_array_element_2 _array_index_2) (`self.quest_history_list`)
        (bind (_year _month _day _hour _minute _second _millisecond) (`KismetMathLibrary.BreakDateTime` (`|GetArrayItem` (`self.quest_history_time`) _array_index_2)))
        (`/Game/MSL_Toolkit/savegame_system/blueprints/bp_msl_savegame_actor.save_string_var` (`/Game/MSL_Toolkit/initial_system/msl_function_library.msl_get_savegame_reference`) "base" "qst" "base" (`.actor_unique_id` (`/Game/MSL_Toolkit/savegame_system/blueprints/bp_msl_identifier_component.get_id` (`.identifier_reference` (`/Game/MSL_Toolkit/initial_system/msl_function_library.msl_get_identifier_component` (`self.GetOwner`))))) "qst_history" (`KismetStringLibrary.Conv_StringToName` (`KismetStringLibrary.Conv_IntToString` _array_index_2)) (`KismetStringLibrary.Concat_StrStr` "?qstid=" (`KismetStringLibrary.Conv_NameToString` _array_element_2) "?qsttime=" (`KismetStringLibrary.Concat_StrStr` (`KismetStringLibrary.Conv_IntToString` _year) "*" (`KismetStringLibrary.Conv_IntToString` _month) "*" (`KismetStringLibrary.Conv_IntToString` _day) "*" (`KismetStringLibrary.Conv_IntToString` _hour) "*" (`KismetStringLibrary.Conv_IntToString` _minute) "*" (`KismetStringLibrary.Conv_IntToString` _second) "*" (`KismetStringLibrary.Conv_IntToString` _millisecond))) false true)))))

(fn `remove_quest`
  (params (quest_unique_id :type Name))
  (locals (local_index :type Integer :default 0) (local_quest_id :type Name) (local_actor :type "/Game/DLG_Tree/dqst_system/blueprints/bp_quest_actor Object Reference"))
  ;[1 1 1] Remove existing quest.
  (set `local.local_quest_id` quest_unique_id)
  (bind (_is_valid _found_index _quest_actor) (`self.get_quest` (`local.local_quest_id`)))
  (if _is_valid
    (set `local.local_index` _found_index)
    (set `local.local_actor` _quest_actor)
    (`|ExecutionSequence`
      (:`then_0`
        (`KismetArrayLibrary.Array_Remove` (`self.quest_list`) (`local.local_index`))
        (`KismetArrayLibrary.Array_Remove` (`self.quest_actors`) (`local.local_index`)))
      (:`then_1`
        (`self.ed_qst_added` (`local.local_actor`) true true)
        (`Actor.K2_DestroyActor` (`local.local_actor`))))))

(fn `set_quest_active`
  (params (quest_unique_id :type Name) (remove_active :type Boolean))
  (locals (local_quest_id :type Name) (local_remove :type Boolean))
  (bind _returnvalue (`KismetArrayLibrary.Array_Find` (`self.active_quest`) (`local.local_quest_id`)))
  ;[1 1 1] Remove active quest from list or add one.
  (set `local.local_quest_id` quest_unique_id)
  (set `local.local_remove` remove_active)
  (if (`local.local_remove`)
    (if (>= _returnvalue 0)
      (`KismetArrayLibrary.Array_Remove` (`self.active_quest`) _returnvalue)
      (bind (_is_valid _found_index _quest_actor) (`self.get_quest` (`local.local_quest_id`)))
      (if _is_valid
        (`/Game/DLG_Tree/dqst_system/blueprints/bp_quest_actor.set_active` _quest_actor false)))
    (elif (< (`self.max_active_quests`) (`KismetArrayLibrary.Array_Length` (`self.active_quest`)))
      (if (`self.auto_remove_active`)
        (`|ExecutionSequence`
          (:`then_0`
            (bind (_is_valid_2 _found_index_2 _quest_actor_2) (`self.get_quest` (`|GetArrayItem` (`self.active_quest`))))
            (if _is_valid_2
              (`/Game/DLG_Tree/dqst_system/blueprints/bp_quest_actor.set_active` _quest_actor_2 false)))
          (:`then_1`
            (`KismetArrayLibrary.Array_Remove` (`self.active_quest`))
            (bind (_is_valid_3 _found_index_3 _quest_actor_3) (`self.get_quest` (`local.local_quest_id`) :!label _label))
            (if _is_valid_3
              (switch `/Game/DLG_Tree/dqst_system/structs/09_enums/enum_quest_result` (`/Game/DLG_Tree/dqst_system/blueprints/bp_quest_actor.quest_status` _quest_actor_3)
                (:`NewEnumerator2`
                  (`KismetArrayLibrary.Array_Add` (`self.active_quest`) (`local.local_quest_id`))
                  (bind (_is_valid_4 _found_index_4 _quest_actor_4) (`self.get_quest` (`local.local_quest_id`)))
                  (if _is_valid_4
                    (`/Game/DLG_Tree/dqst_system/blueprints/bp_quest_actor.set_active` _quest_actor_4 true))))))))
      (else
        (goto _label)))))